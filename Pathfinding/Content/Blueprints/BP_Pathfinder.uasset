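; BP_Pathfinder is an unfinished A* pathfinder that aims to build a path between start and end positions over tagged ground actors.
; On BeginPlay it maps each "Ground" actor's location to the highest cost among its matching gameplay tags.
; The search picks the cheapest frontier position, but neighbor expansion, frontier removal and heuristic are absent.
; Path reconstruction reads CameFrom, which is never filled, and its loop condition appears inverted.
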(event EventBeginPlay
  (bind _path (Variables|Default|GetPath))
  ;[1 1 1] Find all ground objects & their costs
  (bind _outactors (Actor|GetAllActorsOfClasswithTag 0 "Ground"))
  (for _array_element _outactors
    ;[1 1 1] For each ground object, determine its cost
    (Variables|Default|SetCurrentCost 0.0)
    (bind _tagcontainer (GameplayTags|GetOwnedGameplayTags _array_element :!class /Script/GameplayTags.GameplayTagAssetInterface))
    (for _array_element_2 (Variables|Default|GetGroundTypes)
      ;[1 1 1] If the tag is present and the associated cost is higher than the current, increase the current cost
      (if (and (GameplayTags|HasTag _tagcontainer _array_element_2) (> (.Value (Utilities|Map|Find (Variables|Default|GetGroundCosts) _array_element_2)) (Variables|Default|GetCurrentCost)))
        (Variables|Default|SetCurrentCost (.Value (Utilities|Map|Find (Variables|Default|GetGroundCosts) _array_element_2)))))
    (Utilities|Map|Add (Variables|Default|GetPositionCosts) (Transformation|GetActorLocation _array_element) (Variables|Default|GetCurrentCost)))
  ;[1 1 1] Initialize frontier
  (bind _output_get (Variables|Default|SetCurrentPosition (Variables|Default|GetStartPosition)))
  (Utilities|Array|Add (Variables|Default|GetPathFrontier) _output_get)
  ;[1 1 1] Carry out A* pathfinding
  (while (> (Utilities|Array|Length (Variables|Default|GetPathFrontier)) 0)
    ;[1 1 1] Find lowest-cost position along frontier
    (Variables|Default|SetLowestCost 1e+02)
    (for _array_element_3 (Variables|Default|GetPathFrontier)
      (if (and (.ReturnValue (Utilities|Map|Find (Variables|Default|GetPositionCosts) _array_element_3)) (< (.Value (Utilities|Map|Find (Variables|Default|GetPositionCosts) _array_element_3)) (Variables|Default|GetLowestCost)))
        (Variables|Default|SetLowestCost (.Value (Utilities|Map|Find (Variables|Default|GetPositionCosts) _array_element_3)))
        (Variables|Default|SetCurrentPosition _array_element_3))))
  ;[1 1 1] Generate Final Path
  (bind _output_get_2 (Variables|Default|SetCurrentPosition (Variables|Default|GetEndPosition)))
  (Utilities|Array|Add _path _output_get_2)
  (while (Math|Vector|Equal(Vector) (Variables|Default|GetCurrentPosition) (Variables|Default|GetStartPosition) 0.0001)
    (if (.ReturnValue (Utilities|Map|Find (Variables|Default|GetCameFrom) (Variables|Default|GetCurrentPosition)))
      (bind _output_get_3 (Variables|Default|SetCurrentPosition (.Value (Utilities|Map|Find (Variables|Default|GetCameFrom) (Variables|Default|GetCurrentPosition)))))
      (Utilities|Array|Insert _path _output_get_3))))

(event EventTick
  (params (DeltaSeconds :type Float%20%28single-precision%29)))

(fn ConstructionScript)