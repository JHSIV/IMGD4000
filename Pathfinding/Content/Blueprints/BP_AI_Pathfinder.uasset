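; AI controller that plans a weighted grid path to the "Goal" actor at BeginPlay and moves its pawn along it.
; Non-wall "Ground" actors become a string-keyed position map, costed by their highest-cost ground tag.
; An A*-style search expands four-way neighbours by tile cost plus goal distance, without accumulated path cost, then backtracks through CameFrom.
; Tick eases the pawn toward a raised waypoint, advancing every half second.
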(event EventBeginPlay
  (bind _gridspacing (Variables|Default|GetGridSpacing))
  ;[1 1 1] Initialize end position
  (bind _outactors (Actor|GetAllActorswithTag "Goal"))
  (bind _xyposition (CallFunction|GetXYPosition (Utilities|Array|Get(acopy) _outactors)))
  (Variables|Default|SetEndPosition _xyposition)
  ;[1 1 1] Initialize start position
  (bind _xyposition_2 (CallFunction|GetXYPosition self))
  (Variables|Default|SetStartPosition _xyposition_2)
  ;[1 1 1] Find all ground objects & their costs
  (bind _outactors_2 (Actor|GetAllActorswithTag "Ground"))
  (for _array_element _outactors_2
    ;[1 1 1] For each Ground object, determine its cost (Wall objects are ignored)
    (if (not (Actor|ActorHasTag _array_element "Wall"))
      (Variables|Default|SetCurrentCost 0.0)
      (for _array_element_2 (Variables|Default|GetGroundTypes)
        ;[1 1 1] If the tag is present and the associated cost is higher than the current, increase the current cost
        (if (and (Actor|ActorHasTag _array_element (GameplayTags|GetTagName _array_element_2)) (> (.Value (Utilities|Map|Find (Variables|Default|GetGroundCosts) _array_element_2)) (Variables|Default|GetCurrentCost)))
          (Variables|Default|SetCurrentCost (.Value (Utilities|Map|Find (Variables|Default|GetGroundCosts) _array_element_2)))))
      ;[1 1 1] Assign cost to position
      (bind _xyposition_3 (CallFunction|GetXYPosition _array_element))
      (Utilities|Map|Add (Variables|Default|GetPositionCosts) (Utilities|String|ToString(Vector) _xyposition_3) (Variables|Default|GetCurrentCost))))
  ;[1 1 1] Initialize frontier
  (bind _output_get (Variables|Default|SetCurrentPosition (Variables|Default|GetStartPosition)))
  (Utilities|Array|Add (Variables|Default|GetPathFrontier) _output_get)
  ;[1 1 1] Carry out A* pathfinding
  (while (and (> (Utilities|Array|Length (Variables|Default|GetPathFrontier)) 0) (not (Variables|Default|GetEndReached)))
    ;[1 1 1] Explore frontier
    (Variables|Default|SetLowestCost 1e+02)
    (bind _array_element_3 (Utilities|Array|ForEachLoopwithBreak (Variables|Default|GetPathFrontier) :!label _label)
      (:LoopBody
        ;[1 1 1] Break if end position reached
        (if (Math|Vector|Equal(Vector) _array_element_3 (Variables|Default|GetEndPosition) 0.0001)
          (Variables|Default|SetEndReached true)
          (Utilities|Array|Add (Variables|Default|GetPathPositions) _array_element_3)
          (goto _label Break)
          (else
            ;[1 1 1] Find lowest-cost position along frontier
            (if (and (.ReturnValue (Utilities|Map|Find (Variables|Default|GetPositionCosts) (Utilities|String|ToString(Vector) _array_element_3))) (< (+ (.Value (Utilities|Map|Find (Variables|Default|GetPositionCosts) (Utilities|String|ToString(Vector) _array_element_3))) (/ (Math|Vector|Distance(Vector) _array_element_3 (Variables|Default|GetEndPosition)) (Variables|Default|GetGridSpacing))) (Variables|Default|GetLowestCost)))
              (Variables|Default|SetLowestCost (+ (.Value (Utilities|Map|Find (Variables|Default|GetPositionCosts) (Utilities|String|ToString(Vector) _array_element_3))) (/ (Math|Vector|Distance(Vector) _array_element_3 (Variables|Default|GetEndPosition)) (Variables|Default|GetGridSpacing))))
              (Variables|Default|SetCurrentPosition _array_element_3)))))
      (:Completed
        (if (not (Variables|Default|GetEndReached))
          ;[1 1 1] Expand frontier (by checking orthogonally adjacent spaces)
          (for _index (range 0 3)
            (if (and (.ReturnValue (Utilities|Map|Find (Variables|Default|GetPositionCosts) (Utilities|String|ToString(Vector) (Math|Vector|MakeVector (Math|Conversions|ToFloat(Integer) (Math|Float|Round (+ (* (Math|Trig|Cos(Degrees) (* _index 9e+01)) _gridspacing) (.X (Math|Vector|BreakVector (Variables|Default|GetCurrentPosition)))))) (Math|Conversions|ToFloat(Integer) (Math|Float|Round (+ (* _gridspacing (Math|Trig|Sin(Degrees) (* _index 9e+01))) (.Y (Math|Vector|BreakVector (Variables|Default|GetCurrentPosition)))))) (.Z (Math|Vector|BreakVector (Variables|Default|GetCurrentPosition))))))) (not (.ReturnValue (Utilities|Map|Find (Variables|Default|GetCameFrom) (Utilities|String|ToString(Vector) (Math|Vector|MakeVector (Math|Conversions|ToFloat(Integer) (Math|Float|Round (+ (* (Math|Trig|Cos(Degrees) (* _index 9e+01)) _gridspacing) (.X (Math|Vector|BreakVector (Variables|Default|GetCurrentPosition)))))) (Math|Conversions|ToFloat(Integer) (Math|Float|Round (+ (* _gridspacing (Math|Trig|Sin(Degrees) (* _index 9e+01))) (.Y (Math|Vector|BreakVector (Variables|Default|GetCurrentPosition)))))) (.Z (Math|Vector|BreakVector (Variables|Default|GetCurrentPosition)))))))))
              (Utilities|Array|Add (Variables|Default|GetPathFrontier) (Math|Vector|MakeVector (Math|Conversions|ToFloat(Integer) (Math|Float|Round (+ (* (Math|Trig|Cos(Degrees) (* _index 9e+01)) _gridspacing) (.X (Math|Vector|BreakVector (Variables|Default|GetCurrentPosition)))))) (Math|Conversions|ToFloat(Integer) (Math|Float|Round (+ (* _gridspacing (Math|Trig|Sin(Degrees) (* _index 9e+01))) (.Y (Math|Vector|BreakVector (Variables|Default|GetCurrentPosition)))))) (.Z (Math|Vector|BreakVector (Variables|Default|GetCurrentPosition)))))
              (Utilities|Map|Add (Variables|Default|GetCameFrom) (Utilities|String|ToString(Vector) (Math|Vector|MakeVector (Math|Conversions|ToFloat(Integer) (Math|Float|Round (+ (* (Math|Trig|Cos(Degrees) (* _index 9e+01)) _gridspacing) (.X (Math|Vector|BreakVector (Variables|Default|GetCurrentPosition)))))) (Math|Conversions|ToFloat(Integer) (Math|Float|Round (+ (* _gridspacing (Math|Trig|Sin(Degrees) (* _index 9e+01))) (.Y (Math|Vector|BreakVector (Variables|Default|GetCurrentPosition)))))) (.Z (Math|Vector|BreakVector (Variables|Default|GetCurrentPosition))))) (Variables|Default|GetCurrentPosition))))
          ;[1 1 1] Remove current position from the frontier
          (Utilities|Array|RemoveItem (Variables|Default|GetPathFrontier) (Variables|Default|GetCurrentPosition))))))
  ;[1 1 1] Generate Final Path
  (Variables|Default|SetCurrentPosition (Variables|Default|GetEndPosition))
  (while (not (or (Math|Vector|Equal(Vector) (Variables|Default|GetCurrentPosition) (Variables|Default|GetStartPosition) 0.0001) (Variables|Default|GetInvalidPath)))
    (if (.ReturnValue (Utilities|Map|Find (Variables|Default|GetCameFrom) (Utilities|String|ToString(Vector) (Variables|Default|GetCurrentPosition))))
      (bind _output_get_2 (Variables|Default|SetCurrentPosition (.Value (Utilities|Map|Find (Variables|Default|GetCameFrom) (Utilities|String|ToString(Vector) (Variables|Default|GetCurrentPosition))))))
      (Utilities|Array|Insert (Variables|Default|GetPathPositions) _output_get_2)
      (else
        (Variables|Default|SetInvalidPath true)))))

(event EventTick
  (params (DeltaSeconds :type Float%20%28single-precision%29))
  (bind _returnvalue (Pawn|GetControlledPawn))
  (bind _returnvalue_2 (Transformation|GetActorLocation _returnvalue))
  ;[1 1 1] Smoothly step actor along path every second
  (if (or (Variables|Default|GetInvalidPath) (> (Utilities|Array|Length (Variables|Default|GetPathPositions)) 0))
    (bind _output_get (Variables|Default|SetDeltaTime (+ DeltaSeconds (Variables|Default|GetDeltaTime))))
    (Transformation|SetActorLocation _returnvalue (+ _returnvalue_2 (* (/ (- (Math|Vector|MakeVector (.X (Math|Vector|BreakVector (Utilities|Array|Get(acopy) (Variables|Default|GetPathPositions) (Variables|Default|GetPathPositionIndex)))) (.Y (Math|Vector|BreakVector (Utilities|Array|Get(acopy) (Variables|Default|GetPathPositions) (Variables|Default|GetPathPositionIndex)))) (+ (.Z (Math|Vector|BreakVector (Utilities|Array|Get(acopy) (Variables|Default|GetPathPositions) (Variables|Default|GetPathPositionIndex)))) 2e+02)) _returnvalue_2) 0.125) DeltaSeconds)) false false)
    (if (>= _output_get 0.5)
      (Variables|Default|SetDeltaTime (- (Variables|Default|GetDeltaTime) 0.5))
      ;[1 1 1] Advance to next target position, if able
      (if (< (Variables|Default|GetPathPositionIndex) (- (Utilities|Array|Length (Variables|Default|GetPathPositions)) 1))
        (Variables|Default|SetPathPositionIndex (+ (Variables|Default|GetPathPositionIndex) 1))))))

(fn ConstructionScript)

(fn GetXYPosition
  (params (Actor :type Actor%20Object%20Reference))
  (bind _returnvalue (Transformation|GetActorLocation Actor))
  (bind (_x _y) (Math|Vector|BreakVector _returnvalue))
  (return (Math|Vector|MakeVector (Math|Conversions|ToFloat(Integer) (Math|Float|Truncate _x)) (Math|Conversions|ToFloat(Integer) (Math|Float|Truncate _y)) 0.0)))